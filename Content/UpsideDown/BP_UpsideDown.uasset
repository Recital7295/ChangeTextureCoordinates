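; Blueprint actor that periodically flips the rotation of the upside-down material on its static mesh.
; The construction script creates a dynamic instance of M_upsideDown for the mesh and stores it.
; BeginPlay runs an endless delay loop that toggles a boolean, alternating the material's Rotation Angle parameter between half and zero every few seconds.
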(event `self.ReceiveTick`
  (params (DeltaSeconds :type "Float (single-precision)")))

(event `self.ReceiveBeginPlay`
  (bind _dmi_upsidedown (`self.DMI_UpsideDown`))
  (if (`self.Condition`) :!label _label
    (`MaterialInstanceDynamic.SetScalarParameterValue` _dmi_upsidedown "Rotation Angle" 0.5)
    (`KismetSystemLibrary.Delay` 3.0)
    (set `self.Condition` false)
    (goto _label)
    (else
      (`MaterialInstanceDynamic.SetScalarParameterValue` _dmi_upsidedown "Rotation Angle" 0.0)
      (`KismetSystemLibrary.Delay` 3.0)
      (set `self.Condition` true)
      (goto _label))))

(fn `UserConstructionScript`
  (bind _returnvalue (`PrimitiveComponent.CreateDynamicMaterialInstance` (`self.StaticMeshComponent`) 0 "/Game/UpsideDown/M_upsideDown.M_upsideDown" "None"))
  (set `self.DMI_UpsideDown` _returnvalue))