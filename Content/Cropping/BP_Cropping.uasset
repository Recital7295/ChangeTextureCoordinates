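; BP_Cropping is an actor that alternates a mesh's material between normal and cropped views every three seconds.
; The construction script creates a dynamic instance of M_Cropping on the static mesh and stores it as DMIUpsideDown.
; BeginPlay runs an endless delay loop that flips a boolean and sets the UpperLeft and LowerRight vector parameters to either the normal or cropped corner values.
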(event `self.ReceiveBeginPlay`
  (bind _dmi_upsidedown (`self.DMI_UpsideDown`))
  (bind _dmi_upsidedown_2 (`self.DMI_UpsideDown`))
  (if (`self.Condition`) :!label _label
    (`MaterialInstanceDynamic.SetVectorParameterValue` _dmi_upsidedown_2 "UpperLeft" (`self.NormalValue_UL`))
    (`MaterialInstanceDynamic.SetVectorParameterValue` _dmi_upsidedown_2 "LowerRight" (`self.NormalValue_LR`))
    (`KismetSystemLibrary.Delay` 3.0)
    (set `self.Condition` false)
    (goto _label)
    (else
      (`MaterialInstanceDynamic.SetVectorParameterValue` _dmi_upsidedown "UpperLeft" (`self.CroppedValue_UL`))
      (`MaterialInstanceDynamic.SetVectorParameterValue` _dmi_upsidedown "LowerRight" (`self.CroppedValue_LR`))
      (`KismetSystemLibrary.Delay` 3.0)
      (set `self.Condition` true)
      (goto _label))))

(fn `UserConstructionScript`
  (bind _returnvalue (`PrimitiveComponent.CreateDynamicMaterialInstance` (`self.StaticMeshComponent`) 0 "/Game/Cropping/M_Cropping.M_Cropping" "None"))
  (set `self.DMI_UpsideDown` _returnvalue))